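; BP_WallButton is a wall button that makes the player character reach its right hand toward it when nearby.
; On sphere overlap it casts to SandboxCharacter_CMC1, caches its anim Blueprint and sets the right-hand IK target to the button's world location.
; A Timeline drives the IK alpha to blend the reach in, and reverses when an overlap ends.
; No press action or button response is implemented.
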(event `self.SphereCollision.OnComponentBeginOverlap`
  (params (OverlappedComponent :type "PrimitiveComponent Object Reference") (OtherActor :type "Actor Object Reference") (OtherComp :type "PrimitiveComponent Object Reference") (OtherBodyIndex :type Integer) (bFromSweep :type Boolean) (SweepResult :type "HitResult Structure (by ref)"))
  ;[0.03398 0.05961 0.15 0.5] Touch
  (bind _assandbox_character_cmc1 (cast `/Game/V/SandboxCharacter_CMC1` OtherActor))
  (bind _assandbox_character_cmc_abp1 (cast `/Game/V/SandboxCharacter_CMC_ABP1` (`SkeletalMeshComponent.GetAnimInstance` (`Character.Mesh` _assandbox_character_cmc1))))
  (set `self.ABP` _assandbox_character_cmc_abp1)
  (set `/Game/V/SandboxCharacter_CMC_ABP1.Right Hand IK Target` (`SceneComponent.K2_GetComponentLocation` (`self.button`)) (`self.ABP`))
  (bind (_direction _trac_k) (`Timeline|Timeline` :!via `PlayFromStart` :!label _label)
    (:`Update`
      (set `/Game/V/SandboxCharacter_CMC_ABP1.Right Hand IK Alpha` _trac_k (`self.ABP`)))))

(event `self.SphereCollision.OnComponentEndOverlap`
  (params (OverlappedComponent :type "PrimitiveComponent Object Reference") (OtherActor :type "Actor Object Reference") (OtherComp :type "PrimitiveComponent Object Reference") (OtherBodyIndex :type Integer))
  ;[0.1466 0.05673 0.15 0.5] Released
  (goto _label :!via `Reverse`))

(fn `UserConstructionScript`)